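; BP_RCGameInstance is the game instance that starts the server connection and presents the main menu.
; On Init it fetches the server manager and calls InitConnection on it.
; ShowMenu creates the WB_MainMenu widget only when no valid cached instance exists, adds it to the viewport, then switches the first player controller to UI-only input with a visible cursor.
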(event EventInit
  (bind _returnvalue (Class|RCGameInstance|GetServerManager))
  (Class|ServerManager|InitConnection _returnvalue))

(fn ShowMenu
  (bind _returnvalue (Game|GetPlayerController 0))
  (Utilities|IsValid (Variables|Default|GetMainMenuWidget)
    (:Is%20Valid
      _)
    (:Is%20Not%20Valid
      (bind _returnvalue_2 (UserInterface|CreateWidget "/Game/UI/Menu/WB_MainMenu.WB_MainMenu_C" _returnvalue))
      (bind _output_get (Variables|Default|SetMainMenuWidget _returnvalue_2))))
  (UserInterface|Viewport|AddtoViewport _output_get 0)
  (Input|SetInputModeUIOnly _returnvalue 0 "DoNotLock" false)
  (Variables|/Script/Engine.PlayerController|SetbShowMouseCursor _returnvalue true)
  (return))